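; Debug actor that switches the player's camper character to "old movement" tuning when G is pressed.
; Tick polls the key, then overwrites the camper movement component's standing and crawling rotation rates and the spring arm's minimum length and camera lag settings, printing a confirmation.
; There is no toggle back.
; A duplicate setup that also binds the game state's intro-complete callback is disconnected, so it never runs.
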(event `self.ReceiveBeginPlay`)

(event `OnIntroComplete`
  (`/Game/LoggingUtilities/BlueprintLoggingLibrary.PrintString` "Intro Completed" "NewEnumerator1" "LogBlueprintUserMessages" true self))

(event `self.ReceiveTick`
  (params (DeltaSeconds :type "Float (single-precision)"))
  (if (`PlayerController.WasInputKeyJustPressed` (`GameplayStatics.GetPlayerController` 0) "G")
    (bind _asbp_camper_character (cast `/Game/Characters/Campers/Blueprints/BP_Camper_Character` (`GameplayStatics.GetPlayerCharacter` 0)))
    (bind _ascamper_movement_component (cast `CamperMovementComponent` (`Character.CharacterMovement` _asbp_camper_character)))
    (set `CamperMovementComponent._rotationRateWhileCrawling` (struct :`Yaw` 360.0) _ascamper_movement_component)
    (set `CamperMovementComponent._defaultRotationRate` (struct :`Yaw` 360.0) _ascamper_movement_component)
    (bind _dbdspringarm (`/Game/Characters/Campers/Blueprints/BP_Camper_Character.DBDSpringArm` _asbp_camper_character))
    (set `DBDSpringArmComponent.TargetArmMinLength` 45.0 _dbdspringarm)
    (set `DBDSpringArmComponent.ComponenwiseCameraLagSpeed` (6.0 6.0 6.0) _dbdspringarm)
    (set `SpringArmComponent.CameraLagMaxDistance` 75.0 _dbdspringarm)
    (`/Game/LoggingUtilities/BlueprintLoggingLibrary.PrintString` "old movement" "NewEnumerator2" "LogBlueprintUserMessages" true self)))

(fn `UserConstructionScript`)